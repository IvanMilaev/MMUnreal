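; BP_SectionLogic is an actor that builds a row of BP_Section pieces the player edits by keyboard.
; The Add key appends a default section up to a limit, and number keys cycle the matching section through SectionVariant types.
; Each edit calls DrawSections, which destroys all sections and respawns the list between two fixed end types.
; Classes come from a type-to-class map, and bounds extents place pieces edge to edge along X.
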(event EventBeginPlay
  (bind _sections (Variables|Default|Getsections))
  (Input|EnableInput (Game|GetPlayerController 0))
  ;[1 1 1] init
  (Utilities|Array|Add _sections "NewEnumerator0")
  (Utilities|Array|Add _sections "NewEnumerator0")
  (CallFunction|DrawSections))

(event Collision|EventActorBeginOverlap
  (params (OtherActor :type Actor%20Object%20Reference)))

(event EventTick
  (params (DeltaSeconds :type Float%20%28single-precision%29)))

(event Input|KeyboardEvents|Add
  (params (Key :type Key%20Structure :default "None"))
  (bind _sections (Variables|Default|Getsections))
  (:Pressed
    (if (<= (Utilities|Array|Length _sections) 10)
      (Utilities|Array|Add _sections "NewEnumerator0")
      (CallFunction|DrawSections))))

(event Input|KeyboardEvents|1
  (params (Key :type Key%20Structure :default "None"))
  (:Pressed
    (CallFunction|ChangetoSectionB)))

(event Input|KeyboardEvents|9
  (params (Key :type Key%20Structure :default "None"))
  (:Pressed
    (CallFunction|ChangetoSectionB 8)))

(event Input|KeyboardEvents|2
  (params (Key :type Key%20Structure :default "None"))
  (:Pressed
    (CallFunction|ChangetoSectionB 1)))

(event Input|KeyboardEvents|0
  (params (Key :type Key%20Structure :default "None"))
  (:Pressed
    (CallFunction|ChangetoSectionB 9)))

(event Input|KeyboardEvents|3
  (params (Key :type Key%20Structure :default "None"))
  (:Pressed
    (CallFunction|ChangetoSectionB 2)))

(event Input|KeyboardEvents|4
  (params (Key :type Key%20Structure :default "None"))
  (:Pressed
    (CallFunction|ChangetoSectionB 3)))

(event Input|KeyboardEvents|5
  (params (Key :type Key%20Structure :default "None"))
  (:Pressed
    (CallFunction|ChangetoSectionB 4)))

(event Input|KeyboardEvents|6
  (params (Key :type Key%20Structure :default "None"))
  (:Pressed
    (CallFunction|ChangetoSectionB 5)))

(event Input|KeyboardEvents|7
  (params (Key :type Key%20Structure :default "None"))
  (:Pressed
    (CallFunction|ChangetoSectionB 6)))

(event Input|KeyboardEvents|8
  (params (Key :type Key%20Structure :default "None"))
  (:Pressed
    (CallFunction|ChangetoSectionB 7)))

(fn ConstructionScript)

(fn DrawSections
  (bind _sectionsarray (LocalVariables|GetsectionsArray))
  ;[1 1 1] Destroy current section objects
  (bind _outactors (Actor|GetAllActorsOfClass "/Game/dev/blueprints/BP_Section.BP_Section_C"))
  (for _array_element _outactors
    (Actor|DestroyActor _array_element))
  (Utilities|Array|Add _sectionsarray "NewEnumerator3")
  (Utilities|Array|AppendArray _sectionsarray (Variables|Default|Getsections))
  (Utilities|Array|Add _sectionsarray "NewEnumerator4")
  (for _array_element_2 _sectionsarray
    (if (.ReturnValue (Utilities|Map|Find (Variables|Default|GetsectionTypeClasses) _array_element_2))
      _
      (else
        (Development|PrintString (Utilities|GetClassDisplayName (.Value (Utilities|Map|Find (Variables|Default|GetsectionTypeClasses) _array_element_2))))))
    (bind _returnvalue (Game|SpawnActorfromClass (.Value (Utilities|Map|Find (Variables|Default|GetsectionTypeClasses) _array_element_2)) (Math|Transform|MakeTransform (LocalVariables|GetcurrentBorder)) "Undefined" 0 0))
    (Transformation|AddActorLocalOffset _returnvalue (Math|Vector|MakeVector (.X (Math|Vector|BreakVector (.BoxExtent (Collision|GetActorBounds _returnvalue false false)))) 0.0 0.0) false false)
    (LocalVariables|SetcurrentBorder (+ (LocalVariables|GetcurrentBorder) (Math|Vector|MakeVector (* (.X (Math|Vector|BreakVector (.BoxExtent (Collision|GetActorBounds _returnvalue false false)))) 2.0) 0.0 0.0)))))

(fn ChangetoSectionB
  (params (index :type Integer))
  (bind _sectionvariant (LocalVariables|GetsectionVariant))
  (bind _sections (Variables|Default|Getsections))
  (bind _output (Utilities|Array|Get(acopy) _sections index))
  (bind _returnvalue (Utilities|Array|FindItem _sectionvariant _output))
  (if (< index (Utilities|Array|Length _sections))
    (if (== _returnvalue (- (Utilities|Array|Length _sectionvariant) 1))
      (LocalVariables|SetcurentSection (Utilities|Array|Get(acopy) _sectionvariant))
      (else
        (LocalVariables|SetcurentSection (Utilities|Array|Get(acopy) _sectionvariant (+ _returnvalue 1)))))
    (Utilities|Array|SetArrayElem _sections index (LocalVariables|GetcurentSection))
    (CallFunction|DrawSections)))