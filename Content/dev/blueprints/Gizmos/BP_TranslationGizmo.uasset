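; BP_TranslationGizmo is a translation gizmo actor that moves by drag deltas along its local axes.
; On BeginPlay it enables grid use and reads the grid size from BP_GameState.
; Helper functions supply camera transform, orthographic state, a mouse-deprojected ray and the component under the cursor from a complex channel trace.
; ApplyDragDelta offsets the actor without sweeping and forwards the delta through CallOnDeltaReceived; the drag math is not in these graphs.
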(event EventBeginPlay
  (bind _asbp_game_state (Utilities|Casting|CastToBP_GameState (Game|GetGameState)))
  (Variables|Default|SetGameState _asbp_game_state)
  (Variables|Default|SetbGridEnabled true)
  (Variables|Default|SetGridSize (Default|GetGridSize (Variables|Default|GetGameState))))

(event EventApplyDragDelta
  (params (DragDelta :type Vector%20%28by%20ref%29 :default "0, 0, 0"))
  (Transformation|AddActorLocalOffset DragDelta false false)
  (Default|CallOnDeltaReceived DragDelta))

(fn ConstructionScript)

(fn IsOrthoCamera
  (return (Variables|/Script/Engine.PlayerCameraManager|GetbIsOrthographic (Game|GetPlayerCameraManager 0))))

(fn GetRay
  (bind _returnvalue (Game|GetPlayerController 0))
  (bind (_worldlocation _worlddirection) (Game|Player|ConvertMouseLocationToWorldSpace _returnvalue))
  (return _worldlocation _worlddirection))

(fn GetSelectedAxisComponent
  (bind _returnvalue (Game|GetPlayerController 0))
  (bind (_hitresult _returnvalue_2) (Game|Player|GetHitResultUnderCursorbyChannel _returnvalue "TraceTypeQuery3" true))
  (if _returnvalue_2
    (return (.HitComponent (Collision|BreakHitResult _hitresult)))))

(fn GetCameraTransform
  (bind _returnvalue (Game|GetPlayerCameraManager 0))
  (return (Math|Transform|MakeTransform (Camera|GetCameraLocation _returnvalue) (Camera|GetCameraRotation _returnvalue) "1,1,1")))