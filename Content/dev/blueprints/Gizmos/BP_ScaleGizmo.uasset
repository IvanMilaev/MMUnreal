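; BP_ScaleGizmo is a scale gizmo that relays scale deltas through CallOnDeltaReceived.
; On BeginPlay it caches BP_GameState, enables the grid and takes the grid size from it.
; Helper functions supply camera transform, orthographic state and a mouse ray deprojected from player 0.
; Axis picking traces under the cursor and recognizes only components tagged AxisScreen, returning the Screen axis.
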(event EventBeginPlay
  (bind _asbp_game_state (Utilities|Casting|CastToBP_GameState (Game|GetGameState)))
  (Variables|Default|SetGameState _asbp_game_state)
  (Variables|Default|SetbGridEnabled true)
  (Variables|Default|SetGridSize (Default|GetGridSize (Variables|Default|GetGameState))))

(event Collision|EventActorBeginOverlap
  (params (OtherActor :type Actor%20Object%20Reference)))

(event EventTick
  (params (DeltaSeconds :type Float%20%28single-precision%29)))

(event EventApplyScaleDelta
  (params (DeltaScale :type Vector%20%28by%20ref%29 :default "0, 0, 0"))
  (Default|CallOnDeltaReceived DeltaScale))

(fn ConstructionScript)

(fn IsOrthoCamera
  (return (Variables|/Script/Engine.PlayerCameraManager|GetbIsOrthographic (Game|GetPlayerCameraManager 0))))

(fn GetRay
  (bind _returnvalue (Game|GetPlayerController 0))
  (bind (_worldlocation _worlddirection) (Game|Player|ConvertMouseLocationToWorldSpace _returnvalue))
  (return _worldlocation _worlddirection))

(fn GetCameraTransform
  (bind _returnvalue (Game|GetPlayerCameraManager 0))
  (return (Math|Transform|MakeTransform (Camera|GetCameraLocation _returnvalue) (Camera|GetCameraRotation _returnvalue))))

(fn GetSelectedAxisComponent
  (if (Components|ComponentHasTag (.HitComponent (Collision|BreakHitResult (.HitResult (Game|Player|GetHitResultUnderCursorbyChannel (Game|GetPlayerController 0) "TraceTypeQuery3" false)))) "AxisScreen")
    (return (Variables|Default|Getscreen))))