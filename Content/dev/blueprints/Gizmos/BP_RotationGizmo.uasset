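; BP_RotationGizmo is a rotation gizmo with X, Y, Z and arcball handles for mouse-driven rotation.
; It overrides helpers supplying camera transform, orthographic state, mouse ray and sphere radius.
; A complex cursor trace picks the handle from the hit component's first tag.
; Angle deltas rotate the gizmo itself only in one game-state transformation space, then always broadcast; grid size also comes from game state.
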(event EventApplyAngleDelta
  (params (AngleDelta :type Rotator%20%28by%20ref%29 :default "0, 0, 0"))
  (if (Utilities|Enum|Equal(Enum) (.TransformationSpace (Utilities|Struct|BreakTransformState (Variables|/Game/dev/blueprints/BP_GameState.BP_GameState_C|GetTransformation (Variables|Default|GetGamseState)))) "NewEnumerator1")
    (Class|Actor|AddActorWorldRotation AngleDelta))
  (Default|CallOnDeltaReceived AngleDelta))

(event EventBeginPlay
  (bind _asbp_game_state (Utilities|Casting|CastToBP_GameState (Game|GetGameState)))
  (Variables|Default|SetGamseState _asbp_game_state)
  (Variables|Default|SetbGridEnabled true)
  (Variables|Default|SetGridSize (Default|GetGridSize (Variables|Default|GetGamseState))))

(fn ConstructionScript)

(fn GetFreeRotationSphereRadius
  (return 8e+01))

(fn IsOrthoCamera
  (return (Variables|/Script/Engine.PlayerCameraManager|GetbIsOrthographic (Game|GetPlayerCameraManager 0))))

(fn GetCameraTransform
  (bind _returnvalue (Game|GetPlayerCameraManager 0))
  (return (Math|Transform|MakeTransform (Camera|GetCameraLocation _returnvalue) (Camera|GetCameraRotation _returnvalue))))

(fn GetRay
  (bind _returnvalue (Game|GetPlayerController 0))
  (bind (_worldlocation _worlddirection) (Game|Player|ConvertMouseLocationToWorldSpace _returnvalue))
  (return _worldlocation _worlddirection))

(fn GetSelectedAxisComponent
  (bind _returnvalue (Game|GetPlayerController 0))
  (bind (_hitresult _returnvalue_2) (Game|Player|GetHitResultUnderCursorbyChannel _returnvalue "TraceTypeQuery3" true))
  (if _returnvalue_2
    (switch name (Utilities|Array|Get(acopy) (Variables|/Script/Engine.ActorComponent|GetComponentTags (.HitComponent (Collision|BreakHitResult _hitresult))))
      (:AxisX
        (return (Variables|Default|Getrx)))
      (:AxisY
        (return (Variables|Default|Getry)))
      (:AxisZ
        (return (Variables|Default|Getrz)))
      (:AxisXYZ
        (return (Variables|Default|GetArcball))))))